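; Player controller for a Snake game that manages the in-game HUD and the game-over screen.
; On possess, it polls the pawn with a short delay until its snake actor is valid, then creates the HUD showing snake length.
; The snake's food event updates the HUD score.
; Snake destruction swaps the HUD for the game-over widget in Game-and-UI input mode, whose exit click quits the game.
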(event `FoundFood_Event_0`
  (params (Food :type Integer))
  (`/Game/UI/W_GameMain.SetUIScore` (`self.GameMain`) Food))

(event `self.ReceivePossess`
  (params (PossessedPawn :type "Pawn Object Reference"))
  (bind _asplayer_pawn_bp (cast `/Game/PlayerPawnBP` PossessedPawn))
  (bind _snakeactor (`PlayerPawnBase.SnakeActor` _asplayer_pawn_bp))
  (`/Engine/EditorBlueprintResources/StandardMacros.IsValid` _snakeactor :!label _label
    (:`Is Valid`
      (bind _assnake_bp (cast `/Game/SnakeBP` _snakeactor))
      (set `self.Snake Actor` _assnake_bp)
      (bind _returnvalue (`|CreateWidget` "/Game/UI/W_GameMain.W_GameMain_C" self))
      (bind _output_get (set `self.GameMain` _returnvalue))
      (`UserWidget.AddToViewport` _output_get 0)
      (bind _returnvalue_2 (`SnakeBase.GetSnakeLenght` _snakeactor))
      (`/Game/UI/W_GameMain.SetUIScore` (`self.GameMain`) _returnvalue_2)
      (add `self.OnDestroyed` (`self.Snake Actor`) (delegate `OnDestroyed_Event_0`))
      (add `SnakeBase.FoundFood` (`self.Snake Actor`) (delegate `FoundFood_Event_0`)))
    (:`Is Not Valid`
      (`KismetSystemLibrary.Delay` 0.2)
      (goto _label))))

(event `OnDestroyed_Event_0` :!signature `self.OnDestroyed`
  (params (DestroyedActor :type "Actor Object Reference"))
  (`self.K2_DestroyActor` (`self.Snake Actor`))
  (`Widget.RemoveFromParent` (`self.GameMain`))
  (bind _returnvalue (`|CreateWidget` "/Game/UI/W_GameOver.W_GameOver_C" self))
  (bind _output_get (set `self.GameOver` _returnvalue))
  (`UserWidget.AddToViewport` _output_get 0)
  (`WidgetBlueprintLibrary.SetInputMode_GameAndUIEx` self (`self.GameOver`) "DoNotLock" false)
  (add `/Game/UI/W_GameOver.ClickExit` (`self.GameOver`) (delegate `ClickExit_Event_0`)))

(event `ClickExit_Event_0`
  (`KismetSystemLibrary.QuitGame` null "Quit"))

(fn `UserConstructionScript`)